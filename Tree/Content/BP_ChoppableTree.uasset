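; BP_ChoppableTree is a tree that falls when chopped, spawns logs and can respawn as a fresh copy.
; Point damage spawns a BP_TreeHitField, and accumulated Chaos break mass triggers the top's physics fall, then delayed log spawns at its child components.
; A bounds-sized kinematic field above the breakable part sets pieces dynamic while leaving an anchor.
; After the fall, trunk damage accumulates until it destroys the stump, optionally spawning a replacement.
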(event OnChaosBreakEvent(BreakeablePart)
  (params (BreakEvent :type Chaos%20Break%20Event%20Structure%20%28by%20ref%29))
  (bind _exceededthreshold (CallFunction|CalculateMassChoppedandCheckThreshold BreakEvent))
  (if _exceededthreshold
    (Utilities|FlowControl|DoOnce false
      (:Completed
        (Variables|Default|SetTreeHasFallen true)
        (Physics|SetSimulatePhysics (Variables|Default|GetTopPart) true)
        (Utilities|FlowControl|Sequence
          (:then_0
            (Utilities|FlowControl|DelayUntilNextTick)
            (bind _breakeablepart (Variables|Default|GetBreakeablePart)
              (:then
                (Components|DestroyComponent _breakeablepart))
              (:else)))
          (:then_1
            (Utilities|FlowControl|Delay (Variables|StuffToChange|GetDurationBeforeLogsSpawn))
            (CallFunction|SpawnLogs)
            (CallFunction|DestroyActoorandCheckRespawn)))))))

(event Custom|SetDynamic
  ;[0.05127 0.05127 0.05127] The "Set Dynamic" node sometimes makes a sphere that is larger than the geometry. So when it was set as dynamic it immediately falls through the world as it has no remaining static pieces to anchor the parts that are set as dynamic.  Try making that set dynamic size smaller to test. If it falls through, change the bounds and multiply by .a lower value to ensure the sphere size for the set bounds always leaves some as static for the anchor.
  (bind _breakeablepart (Variables|Default|GetBreakeablePart)
    (:then
      (Class|GeometryCollectionComponent|ApplyKinematicField _breakeablepart (.SphereRadius (Collision|GetComponentBounds _breakeablepart)) (Math|Vector|MakeVector (.x (Transformation|GetWorldLocation _breakeablepart)) (.y (Transformation|GetWorldLocation _breakeablepart)) (+ (.z (Transformation|GetWorldLocation _breakeablepart)) (* (.z (.BoxExtent (Collision|GetComponentBounds _breakeablepart))) 2.2)))))
    (:else)))

(event Custom|DestroyActoorAndCheckRespawn
  (if (Variables|StuffToChange|GetDoesRespawn)
    (if (Variables|Default|GetTrunkDestroyed)
      (if (Variables|StuffToChange|GetWhenBaseMeshIsDestroyedDoNotRespawn)
        (Actor|DestroyActor)
        (else
          (Utilities|FlowControl|Delay (Variables|StuffToChange|GetRespawnTime) :!label _label)
          (CallFunction|Respawn)))
      (else
        (goto _label)))
    (else
      (Utilities|FlowControl|RetriggerableDelay 0.0)
      (Actor|DestroyActor))))

(event Custom|Respawn
  (Game|SpawnActorfromClass (Utilities|GetClass self) (Transformation|GetActorTransform) "Undefined" "MultiplyWithRoot" 0 0)
  (Actor|DestroyActor))

(event EventBeginPlay)

(event Game|Damage|EventPointDamage
  (params (Damage :type Float%20%28single-precision%29) (DamageType :type Damage%20Type%20Object%20Reference) (HitLocation :type Vector :default "0, 0, 0") (HitNormal :type Vector :default "0, 0, 0") (HitComponent :type Primitive%20Component%20Object%20Reference) (BoneName :type Name :default "None") (ShotFromDirection :type Vector :default "0, 0, 0") (InstigatedBy :type Controller%20Object%20Reference) (DamageCauser :type Actor%20Object%20Reference) (HitInfo :type Hit%20Result%20Structure%20%28by%20ref%29))
  (CallFunction|SetDynamic)
  (CallFunction|TrunkLogic HitComponent Damage)
  (Game|SpawnActorfromClass "/Game/BP_TreeHitField.BP_TreeHitField_C" (Math|Transform|MakeTransform (.Location (Collision|BreakHitResult HitInfo)) "0, 0, 0" "1.000000,1.000000,1.000000") "Undefined" "MultiplyWithRoot" 0 4e+03 5e+01 4e+01 0))

(fn ConstructionScript
  (CallFunction|SetDynamic))

(fn TrunkLogic
  (params (Hit%20Component :type Object%20Object%20Reference) (Damage :type Float%20%28double-precision%29))
  (bind _spawnthisiftrunkdestroyed (Variables|StufftoChange|GetSpawnThisIfTrunkDestroyed))
  (if (and (== Hit%20Component (Variables|Default|GetTrunk)) (Variables|Default|GetTreeHasFallen))
    (bind _exceededdamagethreshold (CallFunction|CalculateTrunkDamage Damage))
    (if _exceededdamagethreshold
      (Variables|Default|SetTrunkDestroyed true)
      (if (Utilities|IsValidClass _spawnthisiftrunkdestroyed)
        (Game|SpawnActorfromClass _spawnthisiftrunkdestroyed (Transformation|GetWorldTransform (Variables|Default|GetTrunk)) "Undefined" "MultiplyWithRoot" 0 0))
      (Components|DestroyComponent (Variables|Default|GetTrunk))
      (CallFunction|DestroyActoorandCheckRespawn))))

(fn CalculateTrunkDamage
  (params (Damage :type Float%20%28double-precision%29))
  (bind _output_get (Variables|Default|SetDamageDoneToTrunk (+ Damage (Variables|Default|GetDamageDoneToTrunk))))
  (return (>= _output_get (Variables|StuffToChange|GetDamageToDestroyTrunk))))

(fn CalculateMassChoppedandCheckThreshold
  (params (ChaosBreakEvent :type Chaos%20Break%20Event%20Structure))
  (bind _output_get (Variables|Default|SetTotalMassBroken (+ (Variables|Default|GetTotalMassBroken) (.mass ChaosBreakEvent))))
  (Development|PrintString (Utilities|String|ToString(Float) _output_get))
  (return (>= _output_get (Variables|StuffToChange|GetMassRequiredToChopTheTree))))

(fn SpawnLogs
  (bind _array_element (Utilities|Array|ForEachLoopwithBreak (Components|GetChildrenComponents (Variables|Default|GetTopPart) false))
    (:LoopBody
      (bind _result (Math|Integer|IncrementInt (Variables|Default|GetLogsSpawned))
        (:%20%20
          (if (not (>= (- _result 1) (Variables|StufftoChange|GetAmountOfLogsToSpawn)))
            (Game|SpawnActorfromClass (Variables|Default|GetSpawnItWhenTopOfTheTreeIsChopped) (Transformation|GetWorldTransform _array_element) "Undefined" "MultiplyWithRoot" 0 0)))))
    (:Completed
      (Components|DestroyComponent (Variables|Default|GetTopPart)))))